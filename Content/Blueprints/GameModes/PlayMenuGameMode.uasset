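; Game mode for the play menu that displays a vehicle in the level based on vehicle data.
; On BeginPlay it binds an event to the OnVehicleSelected dispatcher.
; ChangeVehicle destroys any previously spawned vehicle, then spawns the class from the supplied VehicleData at the VehicleSpawnLocation actor's position and rotation, keeping a reference for the next swap.
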(event Custom|ChangeVehicle
  (params (VehicleData :type Vehicle%20Data%20Row%20Structure))
  (bind _vehiclespawnlocation (Variables|Default|GetVehicleSpawnLocation))
  (Variables|Default|GetSpawnedVehicle
    (:then
      (Actor|DestroyActor (Variables|Default|GetSpawnedVehicle)))
    (:else
      _))
  (bind _returnvalue (Game|SpawnActorfromClass (.Vehicle (Utilities|Struct|BreakVehicleDataRow VehicleData)) (Math|Transform|MakeTransform (Transformation|GetActorLocation _vehiclespawnlocation) (Transformation|GetActorRotation _vehiclespawnlocation)) "Undefined" 0 0))
  (Variables|Default|SetSpawnedVehicle _returnvalue))

(event EventBeginPlay
  (EventDispatchers|BindEventtoOnVehicleSelected (EventDispatchers|CreateEvent :!event Custom|ChangeVehicle)))

(fn ConstructionScript)