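; Game instance that owns persistent player and common game data, opens the front-end menus and manages multiplayer sessions.
; Init constructs both data objects and assigns the car variants data table.
; Most menus and the loading screen are created once and cached, while the server menu is recreated on each open.
; Hosting creates a session and opens the Lobby level as a listen server; other events join or destroy sessions.
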(event EventOpenMainMenu
  (Variables|Widgets|GetMainMenu
    (:then
      _)
    (:else
      (bind _returnvalue (UserInterface|CreateWidget "/Game/Widgets/MainMenu/MainMenu.MainMenu_C" (Game|GetPlayerController 0)))
      (Variables|Widgets|SetMainMenu _returnvalue)))
  (UserInterface|Viewport|AddtoViewport (Variables|Widgets|GetMainMenu) 0)
  (Variables|/Script/Engine.PlayerController|SetbShowMouseCursor (Game|GetPlayerController 0) true))

(event EventOpenHostMenu
  (Variables|Widgets|GetHostMenu
    (:then
      _)
    (:else
      (bind _returnvalue (UserInterface|CreateWidget "/Game/Widgets/MainMenu/HostMenu.HostMenu_C" (Game|GetPlayerController 0)))
      (Variables|Widgets|SetHostMenu _returnvalue)))
  (UserInterface|Viewport|AddtoViewport (Variables|Widgets|GetHostMenu) 0))

(event EventOpenServerMenu
  (bind _returnvalue (UserInterface|CreateWidget "/Game/Widgets/MainMenu/ServerMenu.ServerMenu_C" (Game|GetPlayerController 0)))
  (UserInterface|Viewport|AddtoViewport _returnvalue 0))

(event EventOpenOptionsMenu
  (Variables|Widgets|GetOptionsMenu
    (:then
      _)
    (:else
      (bind _returnvalue (UserInterface|CreateWidget "/Game/Widgets/MainMenu/OptionsMenu.OptionsMenu_C" (Game|GetPlayerController 0)))
      (Variables|Widgets|SetOptionsMenu _returnvalue)))
  (UserInterface|Viewport|AddtoViewport (Variables|Widgets|GetOptionsMenu) 0))

(event EventShowLoadingScreen
  (Variables|Widgets|GetLoadingScreen
    (:then
      _)
    (:else
      (bind _returnvalue (UserInterface|CreateWidget "/Game/Widgets/MainMenu/LoadingScreen.LoadingScreen_C" (Game|GetPlayerController 0)))
      (Variables|Widgets|SetLoadingScreen _returnvalue)))
  (UserInterface|Viewport|AddtoViewport (Variables|Widgets|GetLoadingScreen) 0))

(event EventLaunchLobby
  (params (NumberOfPlayers :type Integer) (EnableLan :type Boolean) (ServerName :type Text))
  (Variables|Default|SetMaxPlayers NumberOfPlayers)
  (Variables|Default|SetServerName ServerName)
  (CallFunction|ShowLoadingScreen)
  (|Session (Game|GetPlayerController 0) (Variables|Default|GetMaxPlayers) EnableLan
    (:OnSuccess
      (Game|OpenLevel(byName) "Lobby" true "listen"))))

(event EventJoinServer
  (params (Session :type Blueprint%20Session%20Result%20Structure))
  (CallFunction|ShowLoadingScreen)
  (|JoinSession (Game|GetPlayerController 0) Session))

(event EventDestroySession
  (params (PlayerController :type Player%20Controller%20Object%20Reference))
  (|DestroySession PlayerController))

(event EventOpenPlayMenu
  (Variables|Widgets|GetPlayMenu
    (:then
      _)
    (:else
      (bind _returnvalue (UserInterface|CreateWidget "/Game/Widgets/PlayMenu/PlayMenuMain.PlayMenuMain_C" (Game|GetPlayerController 0)))
      (Variables|Widgets|SetPlayMenu _returnvalue)))
  (UserInterface|Viewport|AddtoViewport (Variables|Widgets|GetPlayMenu) 0)
  (Variables|/Script/Engine.PlayerController|SetbShowMouseCursor (Game|GetPlayerController 0) true))

(event EventInit
  (bind _returnvalue (Game|ConstructObjectfromClass "/Script/carzone.PlayerData" self))
  (Variables|Default|SetPlayerData _returnvalue)
  (bind _returnvalue_2 (Game|ConstructObjectfromClass "/Script/carzone.CommonGameData" self))
  (bind _output_get (Variables|Default|SetCommonGameData _returnvalue_2))
  (Variables|/Script/carzone.CommonGameData|SetAllCarsDT _output_get "/Game/DataTables/DT_CarVariants.DT_CarVariants"))

(fn GetMainGameInstance
  (return self))