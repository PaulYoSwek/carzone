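; Vehicle weapon component that spawns and holds the active weapon for a CarBase owner, equipping BP_CratorBlator on BeginPlay.
; SetCurrentWeapon reads the weapon class defaults for its SpawnSocket, spawns it using that body socket's actor-space transform, then attaches it to this component keeping relative transforms.
; A missing socket prints a Dutch error; previous weapons are not destroyed.
; UseWeapon and ReleaseWeapon forward to the active weapon.
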(event Custom|SetCurrentWeapon
  (params (NewParam :type BP%20Weapon%20Base%20Class%20Reference))
  (bind _spawnsocket (Utilities|GetClassDefaults NewParam))
  (bind _ascar_base (Utilities|Casting|CastToCarBase (Components|GetOwner)))
  (if (Transformation|DoesSocketExist (Variables|/Script/carzone.VehicleBase|GetBody _ascar_base) _spawnsocket)
    (bind _returnvalue (Game|SpawnActorfromClass NewParam (Transformation|GetSocketTransform (Variables|/Script/carzone.VehicleBase|GetBody _ascar_base) _spawnsocket "RTS_Actor") "Undefined" (Components|GetOwner) 0))
    (bind _output_get (Variables|Default|SetActiveWeapon _returnvalue))
    (Transformation|AttachComponentToComponent _output_get self _spawnsocket "KeepRelative" "KeepRelative" "KeepRelative" true)
    (else
      (Development|PrintString "Wapen socket niet gevonden! Auto mesh moet Top-,Left-,Right-,Behind- en FrontSocket hebben." true true "(R=0.733333,G=0.026972,B=0.000000,A=1.000000)" 1e+02))))

(event EventBeginPlay
  (CallFunction|SetCurrentWeapon "/Game/Assets/Weapons/MachineGun/Blueprints/BP_CratorBlator.BP_CratorBlator_C"))

(event EventTick
  (params (DeltaSeconds :type Float%20%28single-precision%29)))

(fn UseWeapon
  (Default|ExecuteWeapon (Variables|Default|GetActiveWeapon)))

(fn ReleaseWeapon
  (Default|ReleaseWeapon (Variables|Default|GetActiveWeapon)))