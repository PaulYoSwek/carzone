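; BP_VehicleWeaponryComponent is a vehicle component that manages the vehicle's active weapon.
; On BeginPlay it spawns a boxing gloves weapon owned by the vehicle, stores it as the active weapon, attaches it to itself and offsets it forward.
; UseWeapon forwards the fire request to the active weapon's ExecuteWeapon, while Tick is unused.
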(event EventBeginPlay
  (bind _returnvalue (Game|SpawnActorfromClass "/Game/Assets/Weapons/BoxingGloves/BP_WeaponBoxingGloves.BP_WeaponBoxingGloves_C" (.SpawnTransform (Utilities|GetClassDefaults "/Game/Assets/Weapons/BoxingGloves/BP_WeaponBoxingGloves.BP_WeaponBoxingGloves_C")) "Undefined" (Components|GetOwner) 0))
  (bind _output_get (Variables|Default|SetActiveWeapon _returnvalue))
  (Transformation|AttachComponentToComponent _output_get self "None" "KeepRelative" "KeepRelative" "KeepRelative" true)
  (Transformation|SetRelativeLocation (Variables|/Game/Assets/Weapons/BP_WeaponBase.BP_WeaponBase_C|GetDefaultSceneRoot _output_get) "400.000000, 0, 0" false true))

(event EventTick
  (params (DeltaSeconds :type Float%20%28single-precision%29)))

(fn UseWeapon
  (Default|ExecuteWeapon (Variables|Default|GetActiveWeapon)))