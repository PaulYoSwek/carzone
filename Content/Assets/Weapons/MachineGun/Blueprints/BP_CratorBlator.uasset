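; BP_CratorBlator is a machine gun weapon Blueprint that builds on a parent weapon class and adds a spinning gun.
; ExecuteWeaponTick runs the parent logic, then rolls the Gun component at RotatingSpeed scaled by delta time.
; ReleaseWeapon runs the parent logic and clears IsExecuting.
; Shootbullet is empty, and the event graph holds only disabled placeholder events, so any firing behavior is not defined here.
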(event EventBeginPlay
  (|CallParentFunction) ; This node is disabled and will not be called.\nDrag off pins to build functionality.
)

(event Collision|EventActorBeginOverlap
  (params (OtherActor :type Actor%20Object%20Reference))
  (|CallParentFunction OtherActor) ; This node is disabled and will not be called.\nDrag off pins to build functionality.
)

(event EventTick
  (params (DeltaSeconds :type Float%20%28single-precision%29))
  (|CallParentFunction DeltaSeconds) ; This node is disabled and will not be called.\nDrag off pins to build functionality.
)

(fn ConstructionScript
  (|CallParentFunction))

(fn ExecuteWeaponTick
  (params (DeltaTime :type Float%20%28single-precision%29))
  (|CallParentFunction DeltaTime)
  (Transformation|AddLocalRotation (Variables|Default|GetGun) (Math|Rotator|MakeRotator (* DeltaTime (Variables|Default|GetRotatingSpeed)) 0.0 0.0) false true))

(fn ReleaseWeapon
  (|CallParentFunction)
  (Variables|Default|SetbIsExecuting false))

(fn Shootbullet)