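; Boxing glove weapon that punches with two spring-mounted gloves, alternating between them on each use.
; ExecuteWeapon picks the next spring and glove pair unless a punch is already running.
; ExecuteWeaponTick animates the punch by stretching the spring's X scale while sweeping spring and glove forward, then retracts to the minimum reach.
; Hits by the active glove during the forward stroke push the struck component away from the impact point.
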(event OnComponentHit(Glove2)
  (params (HitComponent :type Primitive%20Component%20Object%20Reference) (OtherActor :type Actor%20Object%20Reference) (OtherComp :type Primitive%20Component%20Object%20Reference) (NormalImpulse :type Vector :default "0, 0, 0") (Hit :type Hit%20Result%20Structure%20%28by%20ref%29))
  (bind (_bblockinghit _binitialoverlap _time _distance _location _impactpoint _normal _impactnormal) (Collision|BreakHitResult Hit))
  (if (and (Variables|Default|GetbGloveGoingForward) (not (Variables|Default|GetbGlove1GetsToPunch)))
    (Class|PrimitiveComponent|AddForceatLocation OtherComp (* (* _impactnormal -1.0) (Variables|Default|GetForce)) _impactpoint "None")))

(event OnComponentHit(Glove1)
  (params (HitComponent :type Primitive%20Component%20Object%20Reference) (OtherActor :type Actor%20Object%20Reference) (OtherComp :type Primitive%20Component%20Object%20Reference) (NormalImpulse :type Vector :default "0, 0, 0") (Hit :type Hit%20Result%20Structure%20%28by%20ref%29))
  (bind (_bblockinghit _binitialoverlap _time _distance _location _impactpoint _normal _impactnormal) (Collision|BreakHitResult Hit))
  (if (and (Variables|Default|GetbGloveGoingForward) (Variables|Default|GetbGlove1GetsToPunch))
    (Class|PrimitiveComponent|AddForceatLocation OtherComp (* (* _impactnormal -1.0) (Variables|Default|GetForce)) _impactpoint "None")))

(event EventBeginPlay
  (|CallParentFunction) ; This node is disabled and will not be called.\nDrag off pins to build functionality.
)

(event Collision|EventActorBeginOverlap
  (params (OtherActor :type Actor%20Object%20Reference))
  (|CallParentFunction OtherActor) ; This node is disabled and will not be called.\nDrag off pins to build functionality.
)

(event EventTick
  (params (DeltaSeconds :type Float%20%28single-precision%29))
  (|CallParentFunction DeltaSeconds) ; This node is disabled and will not be called.\nDrag off pins to build functionality.
)

(fn ConstructionScript
  (|CallParentFunction))

(fn ExecuteWeaponTick
  (params (DeltaTime :type Float%20%28single-precision%29))
  (bind _unitsmovedperscaleincrease (Variables|Default|GetUnitsMovedPerScaleIncrease))
  (bind _currentstrikingspring (Variables|Default|GetCurrentStrikingSpring))
  (bind _currentstrikingspring_2 (Variables|Default|GetCurrentStrikingSpring))
  (bind _punchspeedinscaleperdeltasecond (Variables|Default|GetPunchSpeedInScalePerDeltaSecond))
  (bind _unitsmovedperscaleincrease_2 (Variables|Default|GetUnitsMovedPerScaleIncrease))
  (bind _returnvalue (* DeltaTime _punchspeedinscaleperdeltasecond))
  (bind _relativescale3d (Variables|/Script/Engine.SceneComponent|GetRelativeScale3D _currentstrikingspring))
  (bind _relativescale3d_2 (Variables|/Script/Engine.SceneComponent|GetRelativeScale3D _currentstrikingspring_2))
  (bind _returnvalue_2 (+ _relativescale3d (Math|Vector|MakeVector _returnvalue 0.0 0.0)))
  (bind _returnvalue_3 (* _returnvalue _unitsmovedperscaleincrease))
  (bind _returnvalue_4 (* _returnvalue -1.0))
  (bind _returnvalue_5 (+ _relativescale3d_2 (Math|Vector|MakeVector _returnvalue_4 0.0 0.0)))
  (bind _returnvalue_6 (* _returnvalue_4 _unitsmovedperscaleincrease_2))
  (|CallParentFunction DeltaTime)
  (if (Variables|Default|GetbIsExecuting)
    (if (Variables|Default|GetbGloveGoingForward)
      ;[1 1 1] Glove goes forward
      (Transformation|SetRelativeScale3D _currentstrikingspring _returnvalue_2)
      (Transformation|AddRelativeLocation _currentstrikingspring (Math|Vector|MakeVector _returnvalue_3 0.0 0.0) true false)
      (Transformation|AddRelativeLocation (Variables|Default|GetCurrentStrikingGlove) (Math|Vector|MakeVector _returnvalue_3 0.0 0.0) true false)
      (if (>= (.X (Math|Vector|BreakVector _returnvalue_2)) (Variables|Default|GetMaxPunchingReachInScaleUnits))
        (Variables|Default|SetbGloveGoingForward false))
      (else
        ;[1 1 1] Glove goes backwards
        (Transformation|SetRelativeScale3D _currentstrikingspring_2 _returnvalue_5)
        (Transformation|AddRelativeLocation _currentstrikingspring_2 (Math|Vector|MakeVector _returnvalue_6 0.0 0.0) true false)
        (Transformation|AddRelativeLocation (Variables|Default|GetCurrentStrikingGlove) (Math|Vector|MakeVector _returnvalue_6 0.0 0.0) true false)
        (if (<= (.X (Math|Vector|BreakVector _returnvalue_5)) (Variables|Default|GetMinPunchingReachInScaleUnits))
          (Variables|Default|SetbIsExecuting false))))))

(fn ExecuteWeapon
  (if (not (Variables|Default|GetbIsExecuting))
    (|CallParentFunction)
    (bind _output_get (Variables|Default|SetbGlove1GetsToPunch (not (Variables|Default|GetbGlove1GetsToPunch))))
    (Variables|Default|SetbGloveGoingForward true)
    (if _output_get
      (Variables|Default|SetCurrentStrikingSpring (Variables|Default|GetSpring1))
      (Variables|Default|SetCurrentStrikingGlove (Variables|Default|GetGlove1))
      (else
        (Variables|Default|SetCurrentStrikingSpring (Variables|Default|GetSpring2))
        (Variables|Default|SetCurrentStrikingGlove (Variables|Default|GetGlove2))))))